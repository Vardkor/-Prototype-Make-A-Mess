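; BP_Item is a world pickup item that the first-person player collects on contact.
; The construction script reads its row from DT_ItemList into InternData, sets the static mesh from it and sizes the trigger sphere.
; When a BP_FirstPersonCharacter overlaps the sphere, it passes InternData to the character's AddItems and destroys itself.
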(event OnComponentBeginOverlap(Sphere)
  (params (OverlappedComponent :type Primitive%20Component%20Object%20Reference) (OtherActor :type Actor%20Object%20Reference) (OtherComp :type Primitive%20Component%20Object%20Reference) (OtherBodyIndex :type Integer) (bFromSweep :type Boolean) (SweepResult :type Hit%20Result%20Structure%20%28by%20ref%29))
  (bind _asbp_first_person_character (Utilities|Casting|CastToBP_FirstPersonCharacter OtherActor))
  (Default|AddItems _asbp_first_person_character (Variables|Inventory|GetInternData))
  (Actor|DestroyActor))

(fn ConstructionScript
  (Utilities|FlowControl|Sequence
    (:then_0
      (bind _returnvalue (Utilities|GetDataTableRow "/Game/MakeAMess/Blueprint/Inventaire/Data/DT_ItemList.DT_ItemList" (.RowName (Utilities|Struct|BreakDataTableRowHandle (Variables|Inventory|GetItemDataRow))))
        (:then
          (bind _output_get (Variables|Inventory|SetInternData _returnvalue))
          (Components|StaticMesh|SetStaticMesh (Variables|Default|GetStaticMesh) (.Mesh (Utilities|Struct|BreakS_ItemData _output_get))))))
    (:then_1
      (Components|Sphere|SetSphereRadius (Variables|Default|GetSphere) (Variables|Inventory|GetSphereRadius) true))))